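; BP_Player is a player Blueprint that turns the view through touch drag input.
; A touch press stores the start location, and each move converts the delta from the last point into controller pitch and yaw, scaled by TurnSpeed and frame delta time.
; The overlap event is disabled, and unconnected mesh-setting, print and objective-carrying nodes are left unused.
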(event `InputTouch`
  (params (Location :type "Vector Structure") (FingerIndex :type "ETouchIndex Enum"))
  (bind _returnvalue (`GameplayStatics.GetWorldDeltaSeconds`))
  (:`Pressed`
    (set `self.TouchStart` Location))
  (:`Moved`
    (`self.AddControllerPitchInput` (* (.y (- (`self.TouchStart`) Location)) (`self.TurnSpeed`) _returnvalue))
    (`self.AddControllerYawInput` (* (.x (- (`self.TouchStart`) Location)) (`self.TurnSpeed`) _returnvalue))
    (set `self.TouchStart` Location)))

(fn `UserConstructionScript`)